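; BP_Bg2VRGameMode is a game mode that exposes the level's simulated date and time of day, likely for a VR project.
; SetDateAndTime writes minute, hour, day and month to the level's BP_SunPosition actor, updates the sun, then recaptures the SkyLight so ambient lighting matches.
; GetCurrentDateAndTime reads those values back from the same actor, with both functions locating actors by class at call time.
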(event EventBeginPlay)

(event EventTick
  (params (DeltaSeconds :type Float%20%28single-precision%29)))

(fn ConstructionScript)

(fn SetDateandTime
  (params (Minute :type Integer) (Hour :type Integer) (Day :type Integer) (Month :type Integer))
  (bind _returnvalue (Actor|GetActorOfClass "/SunPosition/BP_SunPosition.BP_SunPosition_C"))
  (Variables|/SunPosition/BP_SunPosition.BP_SunPosition_C|SetMinutes _returnvalue Minute)
  (Variables|/SunPosition/BP_SunPosition.BP_SunPosition_C|SetHours _returnvalue Hour)
  (Variables|/SunPosition/BP_SunPosition.BP_SunPosition_C|SetDay _returnvalue Day)
  (Variables|/SunPosition/BP_SunPosition.BP_SunPosition_C|SetMonth _returnvalue Month)
  (Default|UpdateSun _returnvalue)
  (bind _returnvalue_2 (Actor|GetActorOfClass "/Script/Engine.SkyLight"))
  (Class|SkyLightComponent|RecaptureSky (Variables|/Script/Engine.SkyLight|GetLightComponent _returnvalue_2)))

(fn GetCurrentDateandTime
  (bind _returnvalue (Actor|GetActorOfClass "/SunPosition/BP_SunPosition.BP_SunPosition_C"))
  (return (Variables|/SunPosition/BP_SunPosition.BP_SunPosition_C|GetMinutes _returnvalue) (Variables|/SunPosition/BP_SunPosition.BP_SunPosition_C|GetHours _returnvalue) (Variables|/SunPosition/BP_SunPosition.BP_SunPosition_C|GetDay _returnvalue) (Variables|/SunPosition/BP_SunPosition.BP_SunPosition_C|GetMonth _returnvalue)))